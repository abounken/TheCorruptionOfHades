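; Poseidon crystal pickup that bobs and spins, and can be collected by holding F when a close-combat pawn reaches it underwater.
; Sphere overlap shows the camera-facing prompt and progress bar, enables input and opens a gate.
; Tick tracks hold time into the bar; a full hold passes the gate, makes the Banner interactable and highlighted, awards Poseidon XP and destroys the pickup.
; Item-count quest logic is disconnected.
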(event `self.ReceiveBeginPlay`
  (bind _crystal (`self.Crystal`))
  (set `self.OriginalMat` (`PrimitiveComponent.GetMaterial` (`self.StaticMeshComponent`) 0))
  (bind (_direction _updown) (`Timeline|UpDown`)
    (:`Update`
      (`SceneComponent.K2_SetRelativeTransform` _crystal (`KismetMathLibrary.MakeTransform` (`KismetMathLibrary.MakeVector` 0.0 0.0 _updown) (`SceneComponent.RelativeRotation` _crystal)) false false))))

(event `FinalPickup`
  (bind _banner (`self.Banner`))
  (`/Engine/EditorBlueprintResources/StandardMacros.Gate` true :!label _label
    (:`Exit`
      (set `/Game/Enviornment/Env_BP/Lever2_BP.Interactable` true _banner)
      (`PrimitiveComponent.SetRenderCustomDepth` (`/Game/Enviornment/Env_BP/Lever2_BP.Flag_zeus` _banner) true)
      (bind _asthea_gi (cast `/Game/Characters/Thea/Blueprints/Thea_GI` (`GameplayStatics.GetGameInstance`)))
      (`/Game/Characters/Thea/Blueprints/Thea_GI.AddPoseidonXP` _asthea_gi (`self.PoseidonXP`))
      (`self.K2_DestroyActor`))))

(event `self.Sphere.OnComponentBeginOverlap`
  (params (OverlappedComponent :type "PrimitiveComponent Object Reference") (OtherActor :type "Actor Object Reference") (OtherComp :type "PrimitiveComponent Object Reference") (OtherBodyIndex :type Integer) (bFromSweep :type Boolean) (SweepResult :type "HitResult Structure (by ref)"))
  (if (`KismetMathLibrary.ClassIsChildOf` (`GameplayStatics.GetObjectClass` OtherActor) "/Game/CloseCombat/Blueprints/Player/Pawn_CloseCombat.Pawn_CloseCombat_C")
    (bind _asthea_gi (cast `/Game/Characters/Thea/Blueprints/Thea_GI` (`GameplayStatics.GetGameInstance`)))
    (if (`/Game/Characters/Thea/Blueprints/Thea_GI.IsUnderwater` _asthea_gi)
      (`SceneComponent.SetHiddenInGame` (`self.TextRender`) false false)
      (`SceneComponent.SetHiddenInGame` (`self.InteractBar`) false false)
      (`self.EnableInput` (`GameplayStatics.GetPlayerController` 0))
      (goto _label :!via `Open`))))

(event `self.Sphere.OnComponentEndOverlap`
  (params (OverlappedComponent :type "PrimitiveComponent Object Reference") (OtherActor :type "Actor Object Reference") (OtherComp :type "PrimitiveComponent Object Reference") (OtherBodyIndex :type Integer))
  (if (`KismetMathLibrary.ClassIsChildOf` (`GameplayStatics.GetObjectClass` OtherActor) "/Game/CloseCombat/Blueprints/Player/Pawn_CloseCombat.Pawn_CloseCombat_C")
    (`SceneComponent.SetHiddenInGame` (`self.TextRender`) true false)
    (`SceneComponent.SetHiddenInGame` (`self.InteractBar`) true false)
    (`self.DisableInput` (`GameplayStatics.GetPlayerController` 0))))

(event `self.ReceiveTick`
  (params (DeltaSeconds :type "Float (single-precision)"))
  (bind _textrender (`self.TextRender`))
  ;[1 1 1] TextTurn
  (`SceneComponent.K2_AddLocalRotation` (`self.Crystal`) (struct :`Yaw` 2.3) false false)
  (`SceneComponent.K2_AddLocalRotation` _textrender (struct :`Yaw` 0.4) false false)
  (`SceneComponent.K2_SetWorldRotation` _textrender (`KismetMathLibrary.MakeRotator` 0.0 0.0 (.yaw (`KismetMathLibrary.FindLookAtRotation` (`SceneComponent.K2_GetComponentLocation` _textrender) (`self.K2_GetActorLocation` (`GameplayStatics.GetPlayerCameraManager` 0))))) false false)
  (`self.WidgetTurn`)
  (`self.CheckCharge`)
  (`self.SetWidgetPercentage`))

(event `WidgetTurn`
  (bind _interactbar (`self.InteractBar`))
  ;[1 1 1] WidgetTurn
  (`SceneComponent.K2_AddLocalRotation` _interactbar (struct :`Yaw` 0.4) false false)
  (`SceneComponent.K2_SetWorldRotation` _interactbar (`KismetMathLibrary.MakeRotator` 0.0 0.0 (.yaw (`KismetMathLibrary.FindLookAtRotation` (`SceneComponent.K2_GetComponentLocation` _interactbar) (`self.K2_GetActorLocation` (`GameplayStatics.GetPlayerCameraManager` 0))))) false false))

(event `Key|E`
  (params (Key :type "Key Structure")))

(event `Key|F`
  (params (Key :type "Key Structure"))
  (:`Pressed`
    (set `self.IsCharging` true))
  (:`Released`
    (set `self.IsCharging` false)
    (set `self.HoldTime` 0.0)))

(event `CheckCharge`
  (if (`self.IsCharging`)
    (set `self.HoldTime` (`KismetMathLibrary.FClamp` (`PlayerController.GetInputKeyTimeDown` (`GameplayStatics.GetPlayerController` 0) "F") 0.0 (`self.MaxHold`)))
    (if (>= (`self.HoldTime`) (`self.MaxHold`))
      (set `self.HoldTime` 0.0)
      (set `self.IsCharging` false)
      (`self.FinalPickup`))))

(event `SetWidgetPercentage`
  (bind _aspickup_interact_bar (cast `/Game/Enviornment/Env_props/PickupInteractBar` (`WidgetComponent.GetUserWidgetObject` (`self.InteractBar`))))
  (set `/Game/Enviornment/Env_props/PickupInteractBar.PickupPercent` (`self.HoldTime`) _aspickup_interact_bar))

(event `self.Box1.OnClicked`
  (params (TouchedComponent :type "PrimitiveComponent Object Reference") (ButtonPressed :type "Key Structure"))
  (`KismetSystemLibrary.PrintString` "Hello"))

(fn `UserConstructionScript`
  (`SphereComponent.SetSphereRadius` (`self.Sphere`) (`self.PickupRange`) true))