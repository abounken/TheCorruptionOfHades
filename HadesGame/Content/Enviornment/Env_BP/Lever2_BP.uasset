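; Hold-to-interact quest lever that, once the banner-items quest is done, changes the FlagZeus material and fires a custom lever event.
; Pawn_CloseCombat overlap while interactable shows a camera-facing prompt and progress bar and enables input.
; Tick feeds F hold time to the bar; a full hold with the quest flag set disables interaction and outlines.
; Leftover pickup logic (collectible count, quest update, destroy) sits behind a gate whose FinalPickup trigger is unwired here.
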(event `self.ReceiveBeginPlay`
  (set `self.OriginalMat` (`PrimitiveComponent.GetMaterial` (`self.StaticMeshComponent`) 0))
  (bind _aspickup_interact_bar (cast `/Game/Enviornment/Env_props/PickupInteractBar` (`WidgetComponent.GetUserWidgetObject` (`self.InteractBar`))))
  (bind _output_get (set `/Game/Enviornment/Env_props/PickupInteractBar.PickupMax` (`self.TimeToCharge`) _aspickup_interact_bar))
  (set `self.MaxHold` _output_get))

(event `FinalPickup`
  (`/Engine/EditorBlueprintResources/StandardMacros.Gate` true :!label _label
    (:`Exit`
      (bind _asthea_gi (cast `/Game/Characters/Thea/Blueprints/Thea_GI` (`GameplayStatics.GetGameInstance`)))
      (set `/Game/Characters/Thea/Blueprints/Thea_GI.Type1Collectibles` (+ (`/Game/Characters/Thea/Blueprints/Thea_GI.Type1Collectibles` _asthea_gi) 1) _asthea_gi)
      (bind _asthea_gi_2 (cast `/Game/Characters/Thea/Blueprints/Thea_GI` (`GameplayStatics.GetGameInstance`)))
      (bind _type1collectibles (`/Game/Characters/Thea/Blueprints/Thea_GI.Type1Collectibles` _asthea_gi_2))
      (`/Game/Characters/Thea/Blueprints/Thea_GI.SetCurrentQuest` _asthea_gi_2 (`/Game/Characters/Thea/Blueprints/Thea_GI.CurrentQuestID` _asthea_gi_2) (`/Game/Characters/Thea/Blueprints/Thea_GI.CurrentQuestTitle` _asthea_gi_2) (`KismetStringLibrary.Concat_StrStr` (`KismetStringLibrary.Conv_IntToString` _type1collectibles) "/4 Items Gathered") "" "" "" "" false)
      (if (>= _type1collectibles 4)
        (`/Game/Characters/Thea/Blueprints/Thea_GI.SetCurrentQuest` _asthea_gi_2 0 "A LEVER IS FIXED" "Interact with the lever" "" "" "" "" false))
      (`self.K2_DestroyActor`))))

(event `self.Sphere.OnComponentBeginOverlap`
  (params (OverlappedComponent :type "PrimitiveComponent Object Reference") (OtherActor :type "Actor Object Reference") (OtherComp :type "PrimitiveComponent Object Reference") (OtherBodyIndex :type Integer) (bFromSweep :type Boolean) (SweepResult :type "HitResult Structure (by ref)"))
  (if (`KismetMathLibrary.ClassIsChildOf` (`GameplayStatics.GetObjectClass` OtherActor) "/Game/CloseCombat/Blueprints/Player/Pawn_CloseCombat.Pawn_CloseCombat_C")
    (if (`self.Interactable`)
      (`SceneComponent.SetHiddenInGame` (`self.TextRender`) false false)
      (`SceneComponent.SetHiddenInGame` (`self.InteractBar`) false false)
      (`self.EnableInput` (`GameplayStatics.GetPlayerController` 0))
      (goto _label :!via `Open`))))

(event `HideInfo`
  (`SceneComponent.SetHiddenInGame` (`self.TextRender`) true false :!label _label_2)
  (`SceneComponent.SetHiddenInGame` (`self.InteractBar`) true false))

(event `self.Sphere.OnComponentEndOverlap`
  (params (OverlappedComponent :type "PrimitiveComponent Object Reference") (OtherActor :type "Actor Object Reference") (OtherComp :type "PrimitiveComponent Object Reference") (OtherBodyIndex :type Integer))
  (if (`KismetMathLibrary.ClassIsChildOf` (`GameplayStatics.GetObjectClass` OtherActor) "/Game/CloseCombat/Blueprints/Player/Pawn_CloseCombat.Pawn_CloseCombat_C")
    (goto _label_2)))

(event `self.ReceiveTick`
  (params (DeltaSeconds :type "Float (single-precision)"))
  (bind _textrender (`self.TextRender`))
  ;[1 1 1] TextTurn
  (`SceneComponent.K2_AddLocalRotation` _textrender (struct :`Yaw` 0.4) false false)
  (`SceneComponent.K2_SetWorldRotation` _textrender (`KismetMathLibrary.MakeRotator` 0.0 0.0 (.yaw (`KismetMathLibrary.FindLookAtRotation` (`SceneComponent.K2_GetComponentLocation` _textrender) (`self.K2_GetActorLocation` (`GameplayStatics.GetPlayerCameraManager` 0))))) false false)
  (`self.CheckCharge`)
  (`self.SetWidgetPercentage`))

(event `WidgetTurn`
  (bind _interactbar (`self.InteractBar`))
  ;[1 1 1] WidgetTurn
  (`SceneComponent.K2_AddLocalRotation` _interactbar (struct :`Yaw` 0.4) false false)
  (`SceneComponent.K2_SetWorldRotation` _interactbar (`KismetMathLibrary.MakeRotator` 0.0 0.0 (.yaw (`KismetMathLibrary.FindLookAtRotation` (`SceneComponent.K2_GetComponentLocation` _interactbar) (`self.K2_GetActorLocation` (`GameplayStatics.GetPlayerCameraManager` 0))))) false false))

(event `Key|E`
  (params (Key :type "Key Structure")))

(event `Key|F`
  (params (Key :type "Key Structure"))
  (:`Pressed`
    (set `self.IsCharging` true))
  (:`Released`
    (set `self.IsCharging` false)
    (set `self.HoldTime` 0.0)))

(event `CheckCharge`
  (if (`self.IsCharging`)
    (set `self.HoldTime` (`KismetMathLibrary.FClamp` (`PlayerController.GetInputKeyTimeDown` (`GameplayStatics.GetPlayerController` 0) "F") 0.0 (`self.MaxHold`)))
    (if (>= (`self.HoldTime`) (`self.MaxHold`))
      (set `self.HoldTime` 0.0)
      (set `self.IsCharging` false)
      (bind _asthea_gi (cast `/Game/Characters/Thea/Blueprints/Thea_GI` (`GameplayStatics.GetGameInstance`)))
      (if (`/Game/Characters/Thea/Blueprints/Thea_GI.Quest_Done_BannerItems` _asthea_gi)
        (`PrimitiveComponent.SetMaterial` (`self.Flag_zeus`) 1 "/Game/Enviornment/Assets/Flag/pasted__flagMat.pasted__flagMat")
        (set `self.Interactable` false)
        (`self.HideInfo`)
        (`PrimitiveComponent.SetRenderCustomDepth` (`self.StaticMeshComponent`) false)
        (`PrimitiveComponent.SetRenderCustomDepth` (`self.Cube1`) false)
        (`PrimitiveComponent.SetRenderCustomDepth` (`self.Cube`) false)
        (`PrimitiveComponent.SetRenderCustomDepth` (`self.Flag_zeus`) false)
        (`self.CustomLeverLevelEvent`)))))

(event `SetWidgetPercentage`
  (bind _aspickup_interact_bar (cast `/Game/Enviornment/Env_props/PickupInteractBar` (`WidgetComponent.GetUserWidgetObject` (`self.InteractBar`))))
  (set `/Game/Enviornment/Env_props/PickupInteractBar.PickupPercent` (`self.HoldTime`) _aspickup_interact_bar))

(event `self.Box1.OnClicked`
  (params (TouchedComponent :type "PrimitiveComponent Object Reference") (ButtonPressed :type "Key Structure"))
  (`KismetSystemLibrary.PrintString` "Hello"))

(fn `UserConstructionScript`
  (`SphereComponent.SetSphereRadius` (`self.Sphere`) (`self.PickupRange`) true))