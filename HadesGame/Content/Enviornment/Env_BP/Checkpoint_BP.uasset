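; Checkpoint actor that records a respawn point on the player's Pawn_CloseCombat and spins continuously on Tick.
; When a Pawn_CloseCombat overlaps the sphere trigger, an inactive checkpoint turns green and writes its location and current rotation to the player character.
; It then deactivates the player's previous CurrentCheckpoint, which reverts to red, and registers itself, keeping one active at a time.
; Color changes swap the ring and shield materials and the portal particle template.
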(event `self.ReceiveTick`
  (params (DeltaSeconds :type "Float (single-precision)"))
  (`self.K2_AddActorLocalRotation` (struct :`Yaw` 0.3)))

(event `self.SphereTrigger.OnComponentBeginOverlap`
  (params (OverlappedComponent :type "PrimitiveComponent Object Reference") (OtherActor :type "Actor Object Reference") (OtherComp :type "PrimitiveComponent Object Reference") (OtherBodyIndex :type Integer) (bFromSweep :type Boolean) (SweepResult :type "HitResult Structure (by ref)"))
  (if (`KismetMathLibrary.ClassIsChildOf` (`GameplayStatics.GetObjectClass` OtherActor) "/Game/CloseCombat/Blueprints/Player/Pawn_CloseCombat.Pawn_CloseCombat_C")
    (if (not (`self.Active`))
      (set `self.Active` true)
      (`self.ActivateCheckpoint`))))

(event `ActivateCheckpoint`
  (`self.SetGreenColor`)
  (bind _aspawn_close_combat (cast `/Game/CloseCombat/Blueprints/Player/Pawn_CloseCombat` (`GameplayStatics.GetPlayerCharacter` 0)))
  (set `/Game/CloseCombat/Blueprints/Player/Pawn_CloseCombat.Checkpointed` true _aspawn_close_combat)
  (set `/Game/CloseCombat/Blueprints/Player/Pawn_CloseCombat.CheckpointPosition` (`self.K2_GetActorLocation`) _aspawn_close_combat)
  (set `/Game/CloseCombat/Blueprints/Player/Pawn_CloseCombat.CheckpointRotation` (`self.K2_GetActorRotation`) _aspawn_close_combat)
  (if (not (== (`/Game/CloseCombat/Blueprints/Player/Pawn_CloseCombat.CurrentCheckpoint` _aspawn_close_combat) self))
    (`self.DeactivateCheckpoint` (`/Game/CloseCombat/Blueprints/Player/Pawn_CloseCombat.CurrentCheckpoint` _aspawn_close_combat))
    (set `/Game/CloseCombat/Blueprints/Player/Pawn_CloseCombat.CurrentCheckpoint` self _aspawn_close_combat)))

(event `SetGreenColor`
  (bind _shield (`self.Shield`))
  (`PrimitiveComponent.SetMaterial` (`self.Ring`) 0 "/Game/Enviornment/HadesRingsGlow_Green_Mat.HadesRingsGlow_Green_Mat")
  (`PrimitiveComponent.SetMaterial` _shield 0 "/Game/Enviornment/Shield_Green_Mat.Shield_Green_Mat")
  (`PrimitiveComponent.SetMaterial` _shield 1 "/Game/Enviornment/Shield_Green_Mat.Shield_Green_Mat")
  (`PrimitiveComponent.SetMaterial` _shield 2 "/Game/Enviornment/Shield_Green_Mat.Shield_Green_Mat")
  (`ParticleSystemComponent.SetTemplate` (`self.CheckpointPortal`) "/Game/Enviornment/Portals/CheckpointPortalGreen.CheckpointPortalGreen"))

(event `SetRedColor`
  (bind _shield (`self.Shield`))
  (`PrimitiveComponent.SetMaterial` (`self.Ring`) 0 "/Game/Enviornment/HadesRingsGlow_Red_Mat.HadesRingsGlow_Red_Mat")
  (`PrimitiveComponent.SetMaterial` _shield 0 "/Game/Enviornment/Shield_Mat.Shield_Mat")
  (`PrimitiveComponent.SetMaterial` _shield 1 "/Game/Enviornment/Shield_Mat.Shield_Mat")
  (`PrimitiveComponent.SetMaterial` _shield 2 "/Game/Enviornment/Shield_Mat.Shield_Mat")
  (`ParticleSystemComponent.SetTemplate` (`self.CheckpointPortal`) "/Game/Enviornment/Portals/CheckpointPortal.CheckpointPortal"))

(event `DeactivateCheckpoint`
  (`self.SetRedColor`)
  (set `self.Active` false))

(fn `UserConstructionScript`)