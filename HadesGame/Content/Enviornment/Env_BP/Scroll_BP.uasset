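; Readable scroll pickup that shows its title and content in a HUD widget, optionally maxing the player's XP once.
; A range sphere reveals camera-facing hover text and enables the interaction input, which toggles the widget through a gate.
; Targeted scrolls show an arrow and custom-depth stencil highlight until read.
; Closing the widget, or leaving range after reading, calls a custom level event, with Thea_GI tracking proximity.
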(event `self.ReceiveTick`
  (params (DeltaSeconds :type "Float (single-precision)"))
  (bind _textrender (`self.TextRender`))
  ;[1 1 1] TextTurn
  (`SceneComponent.K2_AddLocalRotation` _textrender (struct :`Yaw` 0.4) false false)
  (`SceneComponent.K2_SetWorldRotation` _textrender (`KismetMathLibrary.MakeRotator` 0.0 0.0 (.yaw (`KismetMathLibrary.FindLookAtRotation` (`SceneComponent.K2_GetComponentLocation` _textrender) (`self.K2_GetActorLocation` (`GameplayStatics.GetPlayerCameraManager` 0))))) false false))

(event `self.ReceiveBeginPlay`
  (if (`self.ScrollTargeted`)
    (`self.TargetScroll`)
    (else
      (`self.UnTargetScroll`))))

(event `InputAction|EnvInteraction`
  (params (Key :type "Key Structure"))
  (:`Pressed`
    (`/Engine/EditorBlueprintResources/StandardMacros.Gate` true :!label _label
      (:`Exit`
        (if (`self.ScrollHUDActive`)
          (`GameplayStatics.PlaySound2D` "/Game/Sounds/SoundPackRPGGames_new/SoundPackCue/ActionsCue/Paper_1_Cue.Paper_1_Cue")
          (`KismetSystemLibrary.PrintString` "Unlock")
          (`Widget.RemoveFromParent` (`self.ScrollHUD`))
          (set `self.ScrollHUDActive` false)
          (`self.CallCustomLevelEvent`)
          (else
            (`GameplayStatics.PlaySound2D` "/Game/Sounds/SoundPackRPGGames_new/SoundPackCue/ActionsCue/Paper_4_Cue.Paper_4_Cue")
            (bind _asthea_gi (cast `/Game/Characters/Thea/Blueprints/Thea_GI` (`GameplayStatics.GetGameInstance`)))
            (if (`/Game/Characters/Thea/Blueprints/Thea_GI.ScrollClose` _asthea_gi)
              (`KismetSystemLibrary.PrintString` "Lock")
              (bind _returnvalue (`|CreateWidget` "/Game/Story/ScrollWidget.ScrollWidget_C"))
              (set `/Game/Story/ScrollWidget.ScrollTitle` (`self.ScrollTitle`) _returnvalue)
              (set `/Game/Story/ScrollWidget.ScrollContent` (`self.ScrollContent`) _returnvalue)
              (bind _output_get (set `self.ScrollHUD` _returnvalue))
              (`UserWidget.AddToViewport` _output_get 0)
              (set `self.ScrollRead` true)
              (set `self.ScrollHUDActive` true)
              (if (`self.IsXPBooster`)
                (`self.GiveXP`)
                (set `self.IsXPBooster` false))
              (`self.UnTargetScroll`))))))))

(event `self.RangeSenser.OnComponentBeginOverlap`
  (params (OverlappedComponent :type "PrimitiveComponent Object Reference") (OtherActor :type "Actor Object Reference") (OtherComp :type "PrimitiveComponent Object Reference") (OtherBodyIndex :type Integer) (bFromSweep :type Boolean) (SweepResult :type "HitResult Structure (by ref)"))
  (if (`KismetMathLibrary.ClassIsChildOf` (`GameplayStatics.GetObjectClass` OtherActor) "/Game/CloseCombat/Blueprints/Player/Pawn_CloseCombat.Pawn_CloseCombat_C")
    (bind _asthea_gi (cast `/Game/Characters/Thea/Blueprints/Thea_GI` (`GameplayStatics.GetGameInstance`)))
    (set `/Game/Characters/Thea/Blueprints/Thea_GI.ScrollClose` true _asthea_gi)
    (`SceneComponent.SetHiddenInGame` (`self.TextRender`) false false)
    (`SceneComponent.SetHiddenInGame` (`self.Plane`) false false)
    (`self.EnableInput` (`GameplayStatics.GetPlayerController` 0))
    (goto _label :!via `Open`)))

(event `self.RangeSenser.OnComponentEndOverlap`
  (params (OverlappedComponent :type "PrimitiveComponent Object Reference") (OtherActor :type "Actor Object Reference") (OtherComp :type "PrimitiveComponent Object Reference") (OtherBodyIndex :type Integer))
  (bind _scrollhud (`self.ScrollHUD`))
  ;[1 1 1] Bug here, check for read
  (if (`KismetMathLibrary.ClassIsChildOf` (`GameplayStatics.GetObjectClass` OtherActor) "/Game/CloseCombat/Blueprints/Player/Pawn_CloseCombat.Pawn_CloseCombat_C")
    (bind _asthea_gi (cast `/Game/Characters/Thea/Blueprints/Thea_GI` (`GameplayStatics.GetGameInstance`)))
    (set `/Game/Characters/Thea/Blueprints/Thea_GI.ScrollClose` false _asthea_gi)
    (`SceneComponent.SetHiddenInGame` (`self.TextRender`) true false)
    (`SceneComponent.SetHiddenInGame` (`self.Plane`) true false)
    ;[1 1 1] Test?
    (`/Engine/EditorBlueprintResources/StandardMacros.IsValid` _scrollhud
      (:`Is Valid`
        (`Widget.RemoveFromParent` _scrollhud))
      (:`Is Not Valid`
        _))
    (set `self.ScrollHUDActive` false)
    ;[1 1 1] Fix?
    (if (`self.ScrollRead`)
      (`KismetSystemLibrary.PrintString` "Unlock")
      (`self.CallCustomLevelEvent`)
      (`self.DisableInput` (`GameplayStatics.GetPlayerController` 0)))))

(event `CallCustomLevelEvent`
  (`self.CustomLevelEvent`))

(event `TargetScroll`
  (bind _scroll (`self.Scroll`))
  (`SceneComponent.SetHiddenInGame` (`self.ArrowCylinder`) false false)
  (`SceneComponent.SetHiddenInGame` (`self.ArrowCone`) false false)
  (`PrimitiveComponent.SetRenderCustomDepth` _scroll true)
  (`PrimitiveComponent.SetCustomDepthStencilValue` _scroll 1))

(event `UnTargetScroll`
  (`SceneComponent.SetHiddenInGame` (`self.ArrowCylinder`) true false)
  (`SceneComponent.SetHiddenInGame` (`self.ArrowCone`) true false)
  (`PrimitiveComponent.SetRenderCustomDepth` (`self.Scroll`) false))

(event `GiveXP`
  (bind _aspawn_close_combat (cast `/Game/CloseCombat/Blueprints/Player/Pawn_CloseCombat` (`GameplayStatics.GetPlayerPawn` 0)))
  (`/Game/CloseCombat/Blueprints/Player/Pawn_CloseCombat.MaxOutXP` _aspawn_close_combat))

(fn `UserConstructionScript`
  (`TextRenderComponent.K2_SetText` (`self.TextRender`) (`self.ScrollOverTitle`))
  (`SphereComponent.SetSphereRadius` (`self.RangeSenser`) (`self.SenserRadius`) true))