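; A falling platform that drops shortly after a Pawn_CloseCombat pawn steps into its Box trigger, then resets.
; It records its spawn transform on BeginPlay.
; On overlap, it waits briefly, prints a debug string and enables physics simulation on the static mesh.
; After a further delay it sets the actor back to the saved transform and turns physics off.
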(event `self.ReceiveBeginPlay`
  (set `self.InitialSpawn` (`self.GetTransform`)))

(event `self.Box.OnComponentBeginOverlap`
  (params (OverlappedComponent :type "PrimitiveComponent Object Reference") (OtherActor :type "Actor Object Reference") (OtherComp :type "PrimitiveComponent Object Reference") (OtherBodyIndex :type Integer) (bFromSweep :type Boolean) (SweepResult :type "HitResult Structure (by ref)"))
  (if (`KismetMathLibrary.ClassIsChildOf` (`GameplayStatics.GetObjectClass` OtherActor) "/Game/CloseCombat/Blueprints/Player/Pawn_CloseCombat.Pawn_CloseCombat_C")
    (`KismetSystemLibrary.Delay` 0.75)
    (`KismetSystemLibrary.PrintString` "Hello")
    (`PrimitiveComponent.SetSimulatePhysics` (`self.StaticMeshComponent`) true)
    (`KismetSystemLibrary.Delay` 4.0)
    (`self.K2_SetActorTransform` (`self.InitialSpawn`))
    (`PrimitiveComponent.SetSimulatePhysics` (`self.StaticMeshComponent`) false)))

(fn `UserConstructionScript`)