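; Treasure chest actor that swings its lid open when something overlaps its Range component and closes it when the overlap ends.
; An Open flag gates both events, and any overlapping actor triggers them without filtering.
; The OpenChest timeline drives the lid's relative pitch, playing from start to open and reversing to close.
; Debug strings print on each change, and a separate CloseChest timeline is left unconnected.
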(event `self.Range.OnComponentBeginOverlap`
  (params (OverlappedComponent :type "PrimitiveComponent Object Reference") (OtherActor :type "Actor Object Reference") (OtherComp :type "PrimitiveComponent Object Reference") (OtherBodyIndex :type Integer) (bFromSweep :type Boolean) (SweepResult :type "HitResult Structure (by ref)"))
  (if (not (`self.Open`))
    (`KismetSystemLibrary.PrintString` "OpenChest")
    (set `self.Open` true)
    (bind (_direction _openlid) (`Timeline|OpenChest` :!via `PlayFromStart` :!label _label)
      (:`Update`
        (`SceneComponent.K2_SetRelativeRotation` (`self.TreasureChest_Lid`) (`KismetMathLibrary.MakeRotator` 0.0 _openlid) false false)))))

(event `self.Range.OnComponentEndOverlap`
  (params (OverlappedComponent :type "PrimitiveComponent Object Reference") (OtherActor :type "Actor Object Reference") (OtherComp :type "PrimitiveComponent Object Reference") (OtherBodyIndex :type Integer))
  (if (`self.Open`)
    (`KismetSystemLibrary.PrintString` "CloseChest")
    (set `self.Open` false)
    (goto _label :!via `Reverse`)))

(fn `UserConstructionScript`)