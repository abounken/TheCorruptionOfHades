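; Breakable vase prop that awards score to the player when its capsule is overlapped.
; The construction script gives each vase a random scale on each axis and picks one of five destructible vase meshes at random.
; The first capsule overlap by any actor applies heavy damage to the DestructibleComponent and adds points to the player's ThirdPersonCharacter Score, with a flag blocking repeats.
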(event `self.ReceiveTick`
  (params (DeltaSeconds :type "Float (single-precision)")))

(event `self.Capsule.OnComponentBeginOverlap`
  (params (OverlappedComponent :type "PrimitiveComponent Object Reference") (OtherActor :type "Actor Object Reference") (OtherComp :type "PrimitiveComponent Object Reference") (OtherBodyIndex :type Integer) (bFromSweep :type Boolean) (SweepResult :type "HitResult Structure (by ref)"))
  (bind _destructiblecomponent (`self.DestructibleComponent`))
  (bind _returnvalue (`SceneComponent.K2_GetComponentLocation` _destructiblecomponent))
  (if (not (`self.Destroyed`))
    (set `self.Destroyed` true)
    (`KismetSystemLibrary.PrintString` "Destroy")
    (`DestructibleComponent.ApplyDamage` _destructiblecomponent 1000.0 _returnvalue _returnvalue 0.0)
    (bind _asthird_person_character (cast `/Game/ThirdPersonBP/Blueprints/ThirdPersonCharacter` (`GameplayStatics.GetPlayerCharacter` 0)))
    (set `/Game/ThirdPersonBP/Blueprints/ThirdPersonCharacter.Score` (+ (`/Game/ThirdPersonBP/Blueprints/ThirdPersonCharacter.Score` _asthird_person_character) 100.0) _asthird_person_character)))

(fn `UserConstructionScript`
  (bind _returnvalue (`KismetMathLibrary.RandomFloatInRange` 37.0 66.0))
  (bind _destructiblecomponent (`self.DestructibleComponent`))
  (`SceneComponent.SetRelativeScale3D` (`self.DestructibleComponent`) (`KismetMathLibrary.MakeVector` _returnvalue _returnvalue _returnvalue))
  (switch `int` (`KismetMathLibrary.RandomIntegerInRange` 0 4)
    (:`Default`
      (`DestructibleComponent.SetDestructibleMesh` _destructiblecomponent "/Game/Enviornment/Env_props/VaseProp1_DM.VaseProp1_DM" :!label _label))
    (:`0`
      (goto _label))
    (:`1`
      (`DestructibleComponent.SetDestructibleMesh` _destructiblecomponent "/Game/Enviornment/Env_props/VaseProp2_DM.VaseProp2_DM"))
    (:`2`
      (`DestructibleComponent.SetDestructibleMesh` _destructiblecomponent "/Game/Enviornment/Env_props/VaseProp3_DM.VaseProp3_DM"))
    (:`3`
      (`DestructibleComponent.SetDestructibleMesh` _destructiblecomponent "/Game/Enviornment/Env_props/VaseProp4_DM.VaseProp4_DM"))
    (:`4`
      (`DestructibleComponent.SetDestructibleMesh` _destructiblecomponent "/Game/Enviornment/Env_props/VaseProp5_DM.VaseProp5_DM"))))