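; Thea_GI appears to be the game instance for the Thea character's game, holding collectible and quest state and handling player death.
; ResetLevelGI clears the collectible count and the read-book quest flag, while SetCurrentQuest stores the active quest's ID, title and four task entries.
; PlayerDeath shows the death widget, pauses the game, reveals the cursor and switches input to UI only.
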(event `ResetLevelGI`
  (set `self.Type1Collectibles` 0)
  (set `self.Quest_Readbook` false))

(event `PlayerDeath`
  (bind _returnvalue (`GameplayStatics.GetPlayerController` 0))
  (bind _returnvalue_2 (`|CreateWidget` "/Game/Enviornment/Env_BP/DiedWidget.DiedWidget_C"))
  (`UserWidget.AddToViewport` _returnvalue_2 0)
  (`GameplayStatics.SetGamePaused` true)
  (set `PlayerController.bShowMouseCursor` true _returnvalue)
  (`WidgetBlueprintLibrary.SetInputMode_UIOnlyEx` _returnvalue _returnvalue_2))

(event `SetCurrentQuest`
  (params (QuestID :type Integer) (QuestTitle :type String) (Task1 :type String) (Task2 :type String) (Task3 :type String) (Task4 :type String) (CurrentQuestTask3 :type String))
  (set `self.CurrentQuestID` QuestID)
  (set `self.CurrentQuestTitle` QuestTitle)
  (set `self.CurrentQuestTask1` Task1)
  (set `self.CurrentQuestTask2` Task2)
  (set `self.CurrentQuestTask3` Task3)
  (set `self.CurrentQuestTask4` Task4))